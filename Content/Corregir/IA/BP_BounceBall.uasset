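; BP_BounceBall is a ball Blueprint that bounces with decreasing strength each time it registers a hit.
; Its Hit event applies the stored NewVar vector to the Ball component as a velocity-change impulse, independent of mass.
; While that vector's Z is positive, each hit then clears X and Y and lowers Z by a fixed step, damping later bounces.
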(event `self.ReceiveHit`
  (params (MyComp :type "PrimitiveComponent Object Reference") (Other :type "Actor Object Reference") (OtherComp :type "PrimitiveComponent Object Reference") (bSelfMoved :type Boolean) (HitLocation :type "Vector Structure") (HitNormal :type "Vector Structure") (NormalImpulse :type "Vector Structure") (Hit :type "HitResult Structure (by ref)"))
  (`PrimitiveComponent.AddImpulse` (`self.Ball`) (`self.NewVar`) "None" true)
  (if (> (`.Z` (`KismetMathLibrary.BreakVector3f` (`self.NewVar`))) 0.0)
    (set `self.NewVar` (`KismetMathLibrary.MakeVector` 0.0 0.0 (- (`.Z` (`KismetMathLibrary.BreakVector3f` (`self.NewVar`))) 100.0)))))

(fn `UserConstructionScript`)