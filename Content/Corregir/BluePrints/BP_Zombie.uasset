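; BP_Zombie is an enemy that wanders between random target points until PawnSensing spots a pawn, then speeds up to chase the player.
; A failed chase move starts a self-repeating attack montage whose notify damages the player via sphere overlap at DamageArrow.
; Point damage halts it for a hit reaction before reducing health.
; Death triggers on the hit after health is depleted, playing an animation and loosening collision.
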(event `self.ReceiveBeginPlay`
  (if (`self.player?`) :!label _label
    _
    (elif (not (`self.Isdead?`))
      (`|AIMoveTo` self (0.0 0.0 0.0) (`KismetArrayLibrary.Array_Random` (`self.TargetPoint`))
        (:`then`
          (`KismetSystemLibrary.Delay` 3.0)
          (goto _label))))))

(event `self.PawnSensing.OnSeePawn`
  (params (Pawn :type "Pawn Object Reference"))
  (set `self.player?` true)
  (if (`self.player?`)
    (if (not (`self.Isdead?`))
      (`self.ChasePlayer`))))

(event `self.ReceivePointDamage`
  (params (Damage :type "Float (single-precision)") (DamageType :type "DamageType Object Reference") (HitLocation :type "Vector Structure") (HitNormal :type "Vector Structure") (HitComponent :type "PrimitiveComponent Object Reference") (BoneName :type Name) (ShotFromDirection :type "Vector Structure") (InstigatedBy :type "Controller Object Reference") (DamageCauser :type "Actor Object Reference") (HitInfo :type "HitResult Structure (by ref)"))
  (if (`self.Isdead?`)
    _
    (elif (<= (`self.Health`) 0.0)
      (`self.Death`)
      (else
        (set `CharacterMovementComponent.MaxWalkSpeed` 0.0 (`self.CharacterMovement`))
        (`|PlayMontage` (`self.Mesh`) "/Game/Corregir/Animations/Zombie_Reaction_Hit_mixamo_com_Montage.Zombie_Reaction_Hit_mixamo_com_Montage"
          (:`then`
            (set `CharacterMovementComponent.MaxWalkSpeed` 60.0 (`self.CharacterMovement`))
            (bind _output_get (set `self.Health` (- (`self.Health`) Damage)))
            (`KismetSystemLibrary.PrintString` (`KismetStringLibrary.Conv_DoubleToString` _output_get))))))))

(event `Death`
  (set `self.Isdead?` true)
  (`MovementComponent.StopMovementImmediately` (`self.CharacterMovement`))
  (`SkeletalMeshComponent.PlayAnimation` (`self.Mesh`) "/Game/Ignore/Enemy/Animatios/zombie_dying.zombie_dying" false)
  (`PrimitiveComponent.SetCollisionResponseToChannel` (`self.CapsuleComponent`) "ECC_Pawn" "ECR_Overlap")
  (`PrimitiveComponent.SetCollisionEnabled` (`self.Mesh`) "NoCollision"))

(event `ChasePlayer`
  (set `CharacterMovementComponent.MaxWalkSpeed` 360.0 (`self.CharacterMovement`))
  (`|AIMoveTo` self (0.0 0.0 0.0) (`GameplayStatics.GetPlayerCharacter` 0)
    (:`OnFail`
      (`self.AttackPlayer`))))

(event `AttackPlayer`
  (`|PlayMontage` (`self.Mesh`) "/Game/Corregir/Animations/zombie_attack_Montage.zombie_attack_Montage"
    (:`OnCompleted`
      (`self.AttackPlayer`))
    (:`OnNotifyBegin`
      (bind (_outactors _returnvalue) (`KismetSystemLibrary.SphereOverlapActors` (`SceneComponent.K2_GetComponentLocation` (`self.DamageArrow`)) 80.0 (`|MakeArray` "ObjectTypeQuery3" :!type "EObjectTypeQuery Enum") "/Game/FirstPerson/Blueprints/BP_FirstPersonCharacter.BP_FirstPersonCharacter_C" (`|MakeArray` self :!type "Actor Object Reference")))
      (if _returnvalue
        (for _array_element _outactors
          (`GameplayStatics.ApplyDamage` _array_element 20.0 (`self.GetController`) self "/Script/Engine.DamageType"))))))

(fn `UserConstructionScript`)