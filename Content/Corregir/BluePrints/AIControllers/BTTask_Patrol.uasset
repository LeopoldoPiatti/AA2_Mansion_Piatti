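; Behavior tree task that makes an AI-controlled pawn patrol by walking forward along its facing direction.
; On execute, it issues a move to a point ahead of the pawn, using the Velocity variable as the distance.
; If that move fails, it falls back to a random reachable point around the pawn.
; The task succeeds when either move completes and fails only when both fail.
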(event `self.ReceiveExecuteAI`
  (params (OwnerController :type "AIController Object Reference") (ControlledPawn :type "Pawn Object Reference"))
  (bind _returnvalue (`Actor.K2_GetActorLocation` ControlledPawn))
  (`|AIMoveTo` ControlledPawn (+ _returnvalue (* (`Actor.GetActorForwardVector` ControlledPawn) (`self.Velocity`))) null 120.0
    (:`OnSuccess`
      (`self.FinishExecute` true))
    (:`OnFail`
      (`|AIMoveTo` ControlledPawn (`NavigationSystemV1.K2_GetRandomReachablePointInRadius` _returnvalue 1000.0 null null) null 120.0
        (:`OnSuccess`
          (`self.FinishExecute` true))
        (:`OnFail`
          (`self.FinishExecute` false))))))