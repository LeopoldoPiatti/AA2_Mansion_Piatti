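; BP_DoorKey_Room_11 is a locked door for Room 11 that opens once the key has been obtained.
; GetKey sets CanOpen, and a player overlapping the trigger box while it is set calls OpenDoor a single time through a DoOnce.
; OpenDoor plays a timeline that swings the door's yaw open and disables its collision as it moves.
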(event `self.Box.OnComponentBeginOverlap`
  (params (OverlappedComponent :type "PrimitiveComponent Object Reference") (OtherActor :type "Actor Object Reference") (OtherComp :type "PrimitiveComponent Object Reference") (OtherBodyIndex :type Integer) (bFromSweep :type Boolean) (SweepResult :type "HitResult Structure (by ref)"))
  (cast `/Game/Corregir/BluePrints/BP_Player` OtherActor)
  (if (`self.canOpen?`)
    (`/Engine/EditorBlueprintResources/StandardMacros.DoOnce` false
      (:`Completed`
        (`self.OpenDoor`)))))

(event `OpenDoor`
  (bind (_direction _doorrotation) (`Timeline|OpenDoorTimeline`)
    (:`Update`
      (`SceneComponent.K2_SetRelativeRotation` (`self.Door`) (`KismetMathLibrary.MakeRotator` 0.0 0.0 (`KismetMathLibrary.Lerp` 0.0 120.0 _doorrotation)) false false)
      (`PrimitiveComponent.SetCollisionEnabled` (`self.Door`) "NoCollision"))))

(event `GetKey`
  (set `self.canOpen?` true))

(fn `UserConstructionScript`)