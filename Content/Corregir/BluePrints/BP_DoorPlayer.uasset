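; BP_DoorPlayer is a swinging door that opens and closes automatically as BP_Player enters and leaves its Box trigger.
; Overlap events call OpenDoor and CloseDoor, which play sounds and run one timeline forward or, after a short delay, in reverse to drive the yaw.
; Each timeline update disables the door's collision, including during closing, so the re-enable on exit is overridden once the reverse starts.
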(event `self.Box.OnComponentBeginOverlap`
  (params (OverlappedComponent :type "PrimitiveComponent Object Reference") (OtherActor :type "Actor Object Reference") (OtherComp :type "PrimitiveComponent Object Reference") (OtherBodyIndex :type Integer) (bFromSweep :type Boolean) (SweepResult :type "HitResult Structure (by ref)"))
  ;[1 1 1] Colision con el jugador
  (cast `/Game/Corregir/BluePrints/BP_Player` OtherActor)
  (`self.OpenDoor`))

(event `self.Box.OnComponentEndOverlap`
  (params (OverlappedComponent :type "PrimitiveComponent Object Reference") (OtherActor :type "Actor Object Reference") (OtherComp :type "PrimitiveComponent Object Reference") (OtherBodyIndex :type Integer))
  ;[1 1 1] Colision con el jugador
  (cast `/Game/Corregir/BluePrints/BP_Player` OtherActor)
  (`self.CloseDoor`)
  (`PrimitiveComponent.SetCollisionEnabled` (`self.Door`) "QueryAndPhysics"))

(event `OpenDoor`
  ;[1 1 1] Mecanica de apertura y cierre
  (`GameplayStatics.PlaySound2D` "/Game/Corregir/Sonidos/SC_Door_Open.SC_Door_Open" 1.0 1.0 0.0 null null)
  (bind (_direction _doorrotation) (`Timeline|OpenDoorTimeline` :!via `PlayFromStart` :!label _label)
    (:`Update`
      (`SceneComponent.K2_SetRelativeRotation` (`self.Door`) (`KismetMathLibrary.MakeRotator` 0.0 0.0 (`KismetMathLibrary.Lerp` 0.0 120.0 _doorrotation)) false false)
      (`PrimitiveComponent.SetCollisionEnabled` (`self.Door`) "NoCollision"))))

(event `CloseDoor`
  ;[1 1 1] Mecanica de apertura y cierre
  (`KismetSystemLibrary.Delay` 0.5)
  (`GameplayStatics.PlaySound2D` "/Game/Corregir/Sonidos/SC_Door_Close.SC_Door_Close" 1.0 1.0 0.0 null null)
  (goto _label :!via `ReverseFromEnd`))

(fn `UserConstructionScript`)